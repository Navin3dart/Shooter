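; BP_Target is a damageable target with a health pool that tips over when its health runs out.
; On BeginPlay it binds to its own any-damage event and fills Health from MaxHealth.
; Each hit subtracts damage with clamping, and at zero a Death timeline rotates the SMTargetGun component 90 degrees on the roll axis.
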(event Custom|OnTakeAnyDamage_Event
  (params (DamagedActor :type Actor%20Object%20Reference) (Damage :type Float%20%28single-precision%29) (DamageType :type Damage%20Type%20Object%20Reference) (InstigatedBy :type Controller%20Object%20Reference) (DamageCauser :type Actor%20Object%20Reference))
  (bind _output_get (Variables|Default|SetHealth (Math|Float|Clamp(Float) (- (Variables|Default|GetHealth) Damage) 0.0 (Variables|Default|GetMaxHealth))))
  (if (== _output_get 0.0)
    (bind _newtrack_0 (Timeline|Death Play)
      (:Update
        (Transformation|SetRelativeRotation (Variables|Default|GetSM_TargetGun) (Math|Rotator|MakeRotator (Math|Float|Lerp 0.0 -9e+01 _newtrack_0) 0.0 0.0) false false)))))

(event EventBeginPlay
  (EventDispatchers|AssignOnTakeAnyDamage (delegate Custom|OnTakeAnyDamage_Event))
  (Variables|Default|SetHealth (Variables|Default|GetMaxHealth)))

(event Collision|EventActorBeginOverlap
  (params (OtherActor :type Actor%20Object%20Reference)))

(event EventTick
  (params (DeltaSeconds :type Float%20%28single-precision%29)))

(fn ConstructionScript)