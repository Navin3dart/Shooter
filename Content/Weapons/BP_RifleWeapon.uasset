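; Rifle weapon actor that keeps its muzzle aim aligned with the screen center by adjusting the player character's aim offsets.
; Two seconds after BeginPlay, Tick traces forward from MuzzleSocket with debug drawing and projects the hit or trace end to screen.
; A feedback loop nudges BP_ShooterBaseCharacter's clamped Yaw and Pitch against the offset from center, easing off as it closes.
; It contains no firing logic.
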(event EventBeginPlay
  (bind _asbp_shooter_base_character (Utilities|Casting|CastToBP_ShooterBaseCharacter (Game|Player|GetPlayerPawn 0)))
  (Variables|Default|SetAs%20BP%20Shooter%20Base%20Character _asbp_shooter_base_character)
  (Utilities|FlowControl|Delay 2.0)
  (Variables|Default|SetCondition true))

(event Collision|EventActorBeginOverlap
  (params (OtherActor :type Actor%20Object%20Reference)))

(event EventTick
  (params (DeltaSeconds :type Float%20%28single-precision%29))
  (bind _returnvalue (Viewport|GetViewportSize))
  (bind _weaponmesh (Variables|Default|GetWeaponMesh))
  (bind _as_bp_shooter_base_character (Variables|Default|GetAs%20BP%20Shooter%20Base%20Character))
  (bind _returnvalue_2 (Transformation|GetSocketTransform _weaponmesh "MuzzleSocket" "RTS_World"))
  (bind _returnvalue_3 (Math|Vector|GetForwardVector (.rotation _returnvalue_2)))
  (bind _returnvalue_4 (* _returnvalue_3 1.5e+04))
  (bind _returnvalue_5 (+ (.location _returnvalue_2) _returnvalue_4))
  (if (Variables|Default|GetCondition)
    (bind (_outhit _returnvalue_6) (Collision|LineTraceByChannel (.location _returnvalue_2) _returnvalue_5 "TraceTypeQuery1" false 0 "ForOneFrame"))
    (Variables|/Game/Player/BP_ShooterBaseCharacter.BP_ShooterBaseCharacter_C|SetYaw _as_bp_shooter_base_character (Math|Float|Clamp(Float) (+ (Variables|/Game/Player/BP_ShooterBaseCharacter.BP_ShooterBaseCharacter_C|GetYaw (Variables|Default|GetAs%20BP%20Shooter%20Base%20Character)) (* (Math|Float|SelectFloat -0.25 0.25 (> (.X (Math|Vector2D|BreakVector2D (/ (.ScreenPosition (Class|GameplayStatics|ProjectWorldtoScreen (Game|GetPlayerController 0) (Math|Vector|SelectVector (.ImpactPoint (Collision|BreakHitResult _outhit)) _returnvalue_5 _returnvalue_6) false)) _returnvalue))) 0.5)) (.x (Class|KismetMathLibrary|ClampAxes2D (/ (Class|KismetMathLibrary|GetAbs2D (- (.ScreenPosition (Class|GameplayStatics|ProjectWorldtoScreen (Game|GetPlayerController 0) (Math|Vector|SelectVector (.ImpactPoint (Collision|BreakHitResult _outhit)) _returnvalue_5 _returnvalue_6) false)) (/ _returnvalue 2.0))) 6.0) 0.0 1.0)))) -45.0 45.0))
    (Variables|/Game/Player/BP_ShooterBaseCharacter.BP_ShooterBaseCharacter_C|SetPitch _as_bp_shooter_base_character (Math|Float|Clamp(Float) (+ (Variables|/Game/Player/BP_ShooterBaseCharacter.BP_ShooterBaseCharacter_C|GetPitch _as_bp_shooter_base_character) (* (Math|Float|SelectFloat 0.25 -0.25 (> (.Y (Math|Vector2D|BreakVector2D (/ (.ScreenPosition (Class|GameplayStatics|ProjectWorldtoScreen (Game|GetPlayerController 0) (Math|Vector|SelectVector (.ImpactPoint (Collision|BreakHitResult _outhit)) _returnvalue_5 _returnvalue_6) false)) _returnvalue))) 0.5)) (.y (Class|KismetMathLibrary|ClampAxes2D (/ (Class|KismetMathLibrary|GetAbs2D (- (.ScreenPosition (Class|GameplayStatics|ProjectWorldtoScreen (Game|GetPlayerController 0) (Math|Vector|SelectVector (.ImpactPoint (Collision|BreakHitResult _outhit)) _returnvalue_5 _returnvalue_6) false)) (/ _returnvalue 2.0))) 6.0) 0.0 1.0)))) -45.0 45.0))))

(fn ConstructionScript)